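; Player character with vehicle-style driving, a tank engine sound and a rotating rune.
; A looping timer at roughly 30 Hz ramps max walk speed up while Forward is held, coasts it down on release, and handles slow reversing.
; Turn sensitivity scales with current speed, and inputs handle camera pitch and a held look-behind flip.
; The timer also plays the rune's rotation timeline, while move presses start engine audio at random offsets.
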(event Custom|30th%20sec
  (bind _returnvalue (Pawn|GetControlRotation :!class /Script/Engine.Pawn))
  (bind _charactermovement (Variables|Character|GetCharacterMovement))
  (bind _returnvalue_2 (Math|Rotator|MakeRotator 0.0 0.0 (.yaw _returnvalue)))
  (bind _returnvalue_3 (Math|Vector|GetForwardVector _returnvalue_2))
  ;[1 1 1] Driving
  (Utilities|FlowControl|Sequence
    (:then_0
      (if (Variables|Default|GetIsForward)
        (if (not (>= (Variables|/Script/Engine.CharacterMovementComponent|GetMaxWalkSpeed (Variables|Character|GetCharacterMovement)) 1.5e+03))
          (Variables|/Script/Engine.CharacterMovementComponent|SetMaxWalkSpeed _charactermovement (+ (Variables|/Script/Engine.CharacterMovementComponent|GetMaxWalkSpeed (Variables|Character|GetCharacterMovement)) 1e+01)))
        (elif (> (Variables|/Script/Engine.CharacterMovementComponent|GetMaxWalkSpeed (Variables|Character|GetCharacterMovement)) 0.0)
          (Pawn|Input|AddMovementInput _returnvalue_3 1.0 false)
          (Variables|/Script/Engine.CharacterMovementComponent|SetMaxWalkSpeed _charactermovement (- (Variables|/Script/Engine.CharacterMovementComponent|GetMaxWalkSpeed (Variables|Character|GetCharacterMovement)) 2e+01)))))
    (:then_1
      (if (Variables|Default|GetIsBackward)
        (Variables|/Script/Engine.CharacterMovementComponent|SetMaxWalkSpeed (Variables|Character|GetCharacterMovement) 1e+02)
        (Pawn|Input|AddMovementInput _returnvalue_3 -1.0 false)
        (Variables|Default|SetSoundVolume 0.5)))
    (:then_2
      ;[1 1 1] Rune Rotation
      (bind _rotate (Timeline|Rotation Play)
        (:Update
          (Transformation|SetRelativeRotation (Variables|Default|Getrune) (Math|Rotator|MakeRotator 0.0 0.0 (* _rotate (Variables|Default|GetAngle))) false false))))))

(event EventTick
  (params (DeltaSeconds :type Float%20%28single-precision%29)))

(event EventBeginPlay
  ;[1 1 1] Starts timer and activates 30th sec every 1/30 of a secnd
  (Utilities|Time|SetTimerbyFunctionName 0 "30th sec" 0.03 true) ; Runs function 30th sec every 0,03 second
)

(event Input|ActionEvents|InputActionBackWard
  (params (Key :type Key%20Structure :default "None"))
  ;[1 1 1] Move and Sound
  (:Pressed
    (Variables|Default|SetIsBackward true)
    (bind _returnvalue (Audio|SpawnSound2D "/Game/Sounds/Tank_moving_sound_effect_1.Tank_moving_sound_effect_1" 0.2 1.0 (Math|Conversions|ToFloat(Integer) (Math|Random|RandomIntegerinRange 0 120)) 0))
    (Variables|Default|Set2D%20 _returnvalue))
  (:Released
    (Variables|Default|SetIsBackward false)
    (Audio|Components|Audio|Stop (Variables|Default|Get2D%20))))

(event Input|ActionEvents|InputActionForward
  (params (Key :type Key%20Structure :default "None"))
  ;[1 1 1] Move and Sound
  (:Pressed
    (Variables|Default|SetIsForward true)
    (bind _returnvalue (Audio|SpawnSound2D "/Game/Sounds/Tank_moving_sound_effect_1.Tank_moving_sound_effect_1" 0.3 1.0 (Math|Conversions|ToFloat(Integer) (Math|Random|RandomIntegerinRange 0 120)) 0))
    (Variables|Default|Set2D%20 _returnvalue))
  (:Released
    (Variables|Default|SetIsForward false)
    (Audio|Components|Audio|Stop (Variables|Default|Get2D%20))))

(event Input|ActionEvents|InputActionThrow
  (params (Key :type Key%20Structure :default "None")))

(event Input|ActionEvents|InputActionFlashBackwards
  (params (Key :type Key%20Structure :default "None"))
  (bind _camera (Variables|Default|GetCamera))
  ;[1 1 1] CamRotate
  (:Pressed
    (Transformation|AddLocalRotation _camera (Math|Rotator|MakeRotator 0.0 0.0 1.8e+02) false false))
  (:Released
    (Transformation|AddLocalRotation _camera (Math|Rotator|MakeRotator 0.0 0.0 -1.8e+02) false false)))

(event Input|AxisEvents|InputAxisCameraY
  (params (AxisValue :type Float%20%28single-precision%29))
  ;[1 1 1] CamRotate
  (Transformation|AddLocalRotation (Variables|Default|GetCamera) (Math|Rotator|MakeRotator 0.0 AxisValue 0.0) false false))

(event Input|AxisEvents|InputAxisTurnRight
  (params (AxisValue :type Float%20%28single-precision%29))
  ;[1 1 1] Turning
  (if (> (Variables|/Script/Engine.CharacterMovementComponent|GetMaxWalkSpeed (Variables|Character|GetCharacterMovement)) 1e+02)
    (if (> (Variables|/Script/Engine.CharacterMovementComponent|GetMaxWalkSpeed (Variables|Character|GetCharacterMovement)) 6e+02)
      (Pawn|Input|AddControllerYawInput AxisValue)
      (else
        (Pawn|Input|AddControllerYawInput (/ AxisValue 4.0))))
    (else
      (Pawn|Input|AddControllerYawInput (/ AxisValue 1e+01)))))

(event Input|AxisEvents|InputAxisMoveForward
  (params (AxisValue :type Float%20%28single-precision%29))
  ;[1 1 1] Driving
  (Pawn|Input|AddMovementInput (Math|Vector|GetForwardVector (Math|Rotator|MakeRotator 0.0 0.0 (.yaw (Pawn|GetControlRotation :!class /Script/Engine.Pawn)))) AxisValue false))

(fn ConstructionScript)

(fn NewFunction0)