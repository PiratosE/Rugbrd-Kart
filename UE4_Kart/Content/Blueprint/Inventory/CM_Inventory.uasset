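; Inventory component that stores content in a fixed-count array of slot structs.
; PrepInv resizes the array to the slot count, followed by a loop with an empty body.
; Addtoinven calls CreateStack, which overwrites the first slot matching an empty zero-quantity struct and always reports success, with no merging or full-inventory check.
; Toggle is an empty stub, and BeginPlay and Tick are unused.
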(event EventBeginPlay)

(event EventTick
  (params (DeltaSeconds :type Float%20%28single-precision%29)))

(fn Addtoinven
  (params (ContentToAdd :type ST%20Slot%20Structure))
  (bind _sucess (CallFunction|CreateStack ContentToAdd))
  (bind _output_get (Variables|Default|SetSucess? _sucess))
  (return _output_get))

(fn PrepInv
  (Utilities|Array|Resize (Variables|Default|GetInventory) (Variables|Default|GetNumberSlots))
  (for _array_element (Variables|Default|GetInventory)
    _))

(fn CreateStack
  (params (ContentToAdd :type ST%20Slot%20Structure))
  (bind _inventory (Variables|Default|GetInventory))
  (Utilities|Array|SetArrayElem _inventory (Utilities|Array|FindItem _inventory (Utilities|Struct|MakeST_Slot "(Texture_2_B563DA2A4DBA2DDF9C1EB3A4A16E0FF8=None,Class_6_3AD9715A4F7B9326556602B3BA374A8A=None)")) ContentToAdd)
  (return true))

(fn Toggle)